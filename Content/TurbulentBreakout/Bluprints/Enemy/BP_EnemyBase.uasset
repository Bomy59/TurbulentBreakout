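; Base enemy Blueprint providing shared helpers for arming an enemy and referencing the player.
; AddWeapon spawns a weapon owned by the enemy with stats copied from its class defaults, attaches it to a given component and tracks it in WeaponArray.
; A setup function caches the player pawn and the enemy's controller.
; IsPlayerVisible always returns false here, and the construction script is empty.
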(fn `Add Weapon`
  (params (`Weapon To Spawn` :type "/Game/TurbulentBreakout/Bluprints/Weapons/WeaponBase/BP_WeaponBase Class Reference") (`Weapon Attach Component` :type "SceneComponent Object Reference"))
  (returns (WeaponRef :type "/Game/TurbulentBreakout/Bluprints/Weapons/WeaponBase/BP_WeaponBase Object Reference") (WeaponRefIndex :type Integer))
  (locals (`Weapon Ref` :type "/Game/TurbulentBreakout/Bluprints/Weapons/WeaponBase/BP_WeaponBase Object Reference"))
  (bind (_weapon_ammo _weaponmaxammo _projectilepeirce _projectilecount _weapon_fire_rate _projectile_base_damage _projectile_damage_multiplier _projectile_spread _projectile_speed _hasinfinetammo _projectiletospawn _shootsoundeffect _noammosoundeffect _weaponreadysoundeffect) (defaults `Object` `Weapon To Spawn`))
  (bind _returnvalue (`|SpawnActorFromClass` `Weapon To Spawn` (`self.GetTransform`) "AlwaysSpawn" "MultiplyWithRoot" self _weapon_ammo _weaponmaxammo _projectilepeirce _projectilecount _weapon_fire_rate _projectile_base_damage _projectile_damage_multiplier _projectile_spread _projectile_speed _hasinfinetammo _projectiletospawn _shootsoundeffect _noammosoundeffect _weaponreadysoundeffect null))
  (bind _output_get (set `local.Weapon Ref` _returnvalue))
  (`SceneComponent.K2_AttachToComponent` (`Actor.RootComponent` _output_get) (`local.Weapon Attach Component`) "None" "SnapToTarget" "SnapToTarget" "KeepWorld" true)
  (if (`KismetArrayLibrary.Array_IsValidIndex` (`self.WeaponArray`))
    (bind _returnvalue_2 (`KismetArrayLibrary.Array_Add` (`self.WeaponArray`) (`local.Weapon Ref`)))
    (return (`local.Weapon Ref`) _returnvalue_2)
    (else
      (set `self.WeaponArray` (`|MakeArray` (`local.Weapon Ref`)))
      (return (`local.Weapon Ref`) 0))))

(fn `Get Player and Controler Ref`
  (bind _returnvalue (`GameplayStatics.GetPlayerPawn` 0))
  (if (`KismetSystemLibrary.IsValid` _returnvalue)
    (`|ExecutionSequence`
      (:`then_1`
        (set `self.PlayerRef` _returnvalue)
        (set `self.ControllerRef` (`self.GetController` self))))))

(fn `Is Player Visible`
  (returns (`Player Visible` :type Boolean))
  (return false))

(fn `UserConstructionScript`)