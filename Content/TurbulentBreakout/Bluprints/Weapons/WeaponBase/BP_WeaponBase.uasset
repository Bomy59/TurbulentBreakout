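; Base weapon Blueprint that fires projectiles, enabling input only when its owner's owner is the player pawn.
; The fire input calls FireStart on Triggered for automatic weapons or Started otherwise.
; FireStart checks equipped state, ammo and cooldown, then spawns projectiles with random yaw, passing damage, speed and pierce, and attaches them to the spawn point.
; FireStop blocks firing until a fire-rate timer calls Can Fire; UpdateAmmo only prints ammo.
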(event `self.ReceiveBeginPlay`
  (if (`self.Is Player Controlled`)
    (`self.EnableInput` (`GameplayStatics.GetPlayerController` 0))))

(event `EnhancedInput|/Game/TurbulentBreakout/Bluprints/Inputs/Actions/IA_WeaponFire`
  (params (ActionValue :type Boolean) (ElapsedSeconds :type "Float (double-precision)") (TriggeredSeconds :type "Float (double-precision)") (InputAction :type "InputAction Object Reference" :default "/Game/TurbulentBreakout/Bluprints/Inputs/Actions/IA_WeaponFire.IA_WeaponFire"))
  (:`Triggered`
    (if (`self.ISAutomatic`)
      (`self.FireStart` :!label _label)))
  (:`Started`
    (if (not (`self.ISAutomatic`))
      (goto _label))))

(fn `Can Fire`
  (set `self.CanShoot` true))

(fn `FireStart`
  (bind _projectile_spread (`self.Projectile Spread`))
  (bind (_returnvalue_roll _returnvalue_pitch _returnvalue_yaw) (`KismetMathLibrary.BreakRotator` (`SceneComponent.K2_GetComponentRotation` (`self.Projectile SpawnPoint`))))
  (if (`self.Equpiped`)
    (if (> (`self.Weapon Ammo`) 0)
      (if (`self.CanShoot`)
        (if (not (`self.HasInfinetAmmo`))
          (set `self.Weapon Ammo` (- (`self.Weapon Ammo`) 1)))
        (for _ (range (`self.ProjectileCount`))
          (bind _returnvalue (`|SpawnActorFromClass` (`self.ProjectileToSpawn`) (`KismetMathLibrary.MakeTransform` (`SceneComponent.K2_GetComponentLocation` (`self.Projectile SpawnPoint`)) (`KismetMathLibrary.MakeRotator` 0.0 0.0 (+ _returnvalue_yaw (`KismetMathLibrary.RandomFloatInRange` _projectile_spread (`KismetMathLibrary.Abs` _projectile_spread))))) "AlwaysSpawn" "MultiplyWithRoot" self (* (`self.Projectile Base Damage`) (`self.Projectile Damage Multiplier`)) (`self.Projectile Speed`) (`self.ProjectilePeirce`) null))
          (if (`KismetSystemLibrary.IsValid` _returnvalue)
            (`SceneComponent.K2_AttachToComponent` (`Actor.RootComponent` _returnvalue) (`self.Projectile SpawnPoint`) "None" "KeepWorld" "KeepWorld" "KeepWorld" false)
            (`GameplayStatics.PlaySoundAtLocation` (`self.ShootSoundEffect`) (`self.K2_GetActorLocation`) (struct) 1.0 1.0 0.0 null null null null)))
        (`self.FireStop`))
      (else
        (`GameplayStatics.PlaySoundAtLocation` (`self.NoAmmoSoundEffect`) (`self.K2_GetActorLocation`) (struct) 1.0 1.0 0.0 null null null null)))))

(fn `FireStop`
  (if (`self.Equpiped`)
    (set `self.CanShoot` false)
    (`KismetSystemLibrary.K2_SetTimer` null "Can Fire" (`self.Weapon Fire Rate`))))

(fn `Is Player Controlled`
  (returns (IsPlayer :type Boolean))
  (bind _returnvalue (`self.GetOwner`))
  (if (`KismetSystemLibrary.IsValid` _returnvalue)
    (bind _output_get (set `self.Is Player` (== (`self.GetOwner` _returnvalue) (`GameplayStatics.GetPlayerPawn` 0))))
    (return _output_get)))

(fn `UpdateAmmo`
  (if (not (`self.HasInfinetAmmo`))
    (`KismetSystemLibrary.PrintString` (`KismetStringLibrary.Conv_IntToString` (`self.Weapon Ammo`)))))

(fn `UserConstructionScript`)