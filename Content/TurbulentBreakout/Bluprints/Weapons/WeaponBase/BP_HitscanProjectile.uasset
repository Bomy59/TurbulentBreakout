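; Hitscan laser weapon projectile that fires a single shot one second after spawning.
; A long visibility line trace along the laser effect's forward vector stores the hit actor, scales the beam by hit distance and moves the impact effect to the hit point.
; The stored target takes FinalDamage, cut to a quarter when piercing, which also schedules a Destroy Lazer timer not defined here.
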(event `self.ReceiveBeginPlay`
  (`KismetSystemLibrary.K2_SetTimer` null "Firelazer" 1.0))

(event `Firelazer`
  (`|ExecutionSequence`
    (:`then_0`
      (`self.Create Lazer`))
    (:`then_1`
      (`self.DamageTarget`))))

(fn `Create Lazer`
  (bind _eff_lazer (`self.EFF_Lazer`))
  (bind _returnvalue (`SceneComponent.K2_GetComponentLocation` _eff_lazer))
  (bind _outhit (`KismetSystemLibrary.LineTraceSingle` :`Start` _returnvalue :`End` (+ _returnvalue (* (`SceneComponent.GetForwardVector` _eff_lazer) 9000000.0)) :`TraceChannel` "TraceTypeQuery1" :`DrawDebugType` "ForOneFrame"))
  (set `self.Target` (`.HitActor` (`GameplayStatics.BreakHitResult` _outhit)))
  (`FXSystemComponent.SetVectorParameter` (`self.EFF_Lazer`) "Vector" (`KismetMathLibrary.MakeVector` (* (`.Distance` (`GameplayStatics.BreakHitResult` _outhit)) 5.0)))
  (`SceneComponent.K2_SetWorldLocation` (`self.EFF_LazerImpact`) (`.Location` (`GameplayStatics.BreakHitResult` _outhit)) false true))

(fn `DamageTarget`
  (bind _final_damage (`self.Final Damage`))
  (if (`KismetSystemLibrary.IsValid` (`self.Target`))
    (`GameplayStatics.ApplyDamage` (`self.Target`) (select `bool` (`self.CanPeirce`) :`false` _final_damage :`true` (* _final_damage 0.25)) null self)
    (if (`self.CanPeirce`)
      (`KismetSystemLibrary.K2_SetTimer` null "Destroy Lazer" 1.0))))

(fn `UserConstructionScript`
  (`parent.UserConstructionScript`))