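; Base projectile actor for weapons that flies forward and damages the actors it overlaps.
; Each Tick, MoveProjectile advances it along its root's forward vector by ProjectileSpeed using a swept transform, without delta-time scaling.
; Overlaps apply FinalDamage and use up a Peirce count, destroying the projectile once none remain, while any Hit event destroys it immediately.
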(event `self.ReceiveTick`
  (params (DeltaSeconds :type "Float (single-precision)"))
  (`self.Move Projectile`))

(event `self.ReceiveHit`
  (params (MyComp :type "PrimitiveComponent Object Reference") (Other :type "Actor Object Reference") (OtherComp :type "PrimitiveComponent Object Reference") (bSelfMoved :type Boolean) (HitLocation :type "Vector Structure") (HitNormal :type "Vector Structure") (NormalImpulse :type "Vector Structure") (Hit :type "HitResult Structure (by ref)"))
  (`self.K2_DestroyActor`))

(event `self.ReceiveActorBeginOverlap`
  (params (OtherActor :type "Actor Object Reference"))
  (`GameplayStatics.ApplyDamage` OtherActor (`self.Final Damage`))
  (if (> (`self.Peirce`) 0)
    (set `self.Peirce` (- (`self.Peirce`) 1))
    (else
      (`self.K2_DestroyActor`))))

(fn `Move Projectile`
  (bind (_returnvalue_location _returnvalue_rotation _returnvalue_scale) (`KismetMathLibrary.BreakTransform` (`self.GetTransform`)))
  (`self.K2_SetActorTransform` (`KismetMathLibrary.MakeTransform` (+ (* (`self.Projectile Speed`) (`SceneComponent.GetForwardVector` (`self.DefaultSceneRoot`))) _returnvalue_location) _returnvalue_rotation _returnvalue_scale) true))

(fn `UserConstructionScript`)