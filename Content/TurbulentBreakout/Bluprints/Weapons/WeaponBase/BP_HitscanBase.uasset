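; Base Blueprint for hitscan weapons that traces the shot line and fits the projectile trail and impact to it.
; CreateTrail runs a very long line trace forward from the ProjectileTrail component, with one-frame debug drawing, and stores the hit actor as Target.
; The hit distance feeds the trail's vector parameter, and ProjectileImpact, when valid, teleports to the hit location.
; No damage is applied here.
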(fn `Create Trail`
  (bind _projectile_impact (`self.Projectile Impact`))
  (bind _projectile_trail (`self.Projectile Trail`))
  (bind _returnvalue (`SceneComponent.K2_GetComponentLocation` _projectile_trail))
  (bind _outhit (`KismetSystemLibrary.LineTraceSingle` :`Start` _returnvalue :`End` (+ _returnvalue (* (`SceneComponent.GetForwardVector` _projectile_trail) 9000000.0)) :`TraceChannel` "TraceTypeQuery3" :`DrawDebugType` "ForOneFrame"))
  (set `self.Target` (`.HitActor` (`GameplayStatics.BreakHitResult` _outhit)))
  (`FXSystemComponent.SetVectorParameter` (`self.Projectile Trail`) "Vector" (`KismetMathLibrary.MakeVector` (`.Distance` (`GameplayStatics.BreakHitResult` _outhit))))
  (if (`KismetSystemLibrary.IsValid` _projectile_impact)
    (`SceneComponent.K2_SetWorldLocation` _projectile_impact (`.Location` (`GameplayStatics.BreakHitResult` _outhit)) false true)))

(fn `UserConstructionScript`
  (`parent.UserConstructionScript`))