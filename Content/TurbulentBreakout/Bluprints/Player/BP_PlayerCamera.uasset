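; Player camera actor that turns look input, scaled by sensitivity, into movement of a Cursor component kept within a maximum distance of the actor's root.
; Each move first line-traces on the Camera channel from the root toward the proposed cursor position, at root height.
; Unobstructed moves apply X and Y separately, each with its own range check.
; A hit snaps the cursor to the impact's trace location if within range.
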(event `self.ReceiveBeginPlay`
  (`self.EnableInput` (`GameplayStatics.GetPlayerController` 0)))

(event `EnhancedInput|/Game/TurbulentBreakout/Bluprints/Input/Actions/IA_Look`
  (params (ActionValue :type "Vector2D Structure") (ElapsedSeconds :type "Float (double-precision)") (TriggeredSeconds :type "Float (double-precision)") (InputAction :type "InputAction Object Reference" :default "/Game/TurbulentBreakout/Bluprints/Input/Actions/IA_Look.IA_Look"))
  (:`Triggered`
    (`self.Move Cursor` (* ActionValue_X (`self.Sensitivity`)) (* ActionValue_Y (`self.Sensitivity`)))))

(fn `Get Distance`
  (params (`X/Y` :type Boolean) (Input :type "Float (double-precision)"))
  (returns (ReturnValue :type "Float (double-precision)"))
  (bind (_returnvalue_x _returnvalue_y _returnvalue_z) (`KismetMathLibrary.BreakVector` (`SceneComponent.K2_GetComponentLocation` (`self.Cursor`))))
  (return (`KismetMathLibrary.Vector_Distance` (`KismetMathLibrary.MakeVector` (+ (select `bool` (`local.X/Y`) :`true` (`local.Input`)) _returnvalue_x) (+ (select `bool` (`local.X/Y`) :`false` (`local.Input`)) _returnvalue_y) _returnvalue_z) (`SceneComponent.K2_GetComponentLocation` (`Actor.RootComponent` (`ActorComponent.GetOwner` (`self.DefaultSceneRoot`)))))))

(fn `Move Cursor`
  (params (MouseX :type "Float (double-precision)") (MouseY :type "Float (double-precision)"))
  (bind (_returnvalue_x _returnvalue_y) (`KismetMathLibrary.BreakVector` (`SceneComponent.K2_GetComponentLocation` (`self.Cursor`))))
  (bind (_returnvalue_x_2 _returnvalue_y_2 _returnvalue_z) (`KismetMathLibrary.BreakVector` (`SceneComponent.K2_GetComponentLocation` (`Actor.RootComponent` (`self.GetOwner`)))))
  (bind _outhit (`KismetSystemLibrary.LineTraceSingle` :`Start` (`KismetMathLibrary.MakeVector` _returnvalue_x_2 _returnvalue_y_2 _returnvalue_z) :`End` (`KismetMathLibrary.MakeVector` (+ (`local.MouseX`) _returnvalue_x) (+ (`local.MouseY`) _returnvalue_y) _returnvalue_z) :`TraceChannel` "TraceTypeQuery2" :`DrawDebugType` "ForOneFrame" :`bIgnoreSelf` false))
  (if (not (`KismetSystemLibrary.IsValid` (`.HitActor` (`GameplayStatics.BreakHitResult` _outhit))))
    (`|ExecutionSequence`
      (:`then_0`
        (if (<= (`self.Get Distance` true (`local.MouseX`)) (`self.MaxDistance`))
          (`SceneComponent.K2_AddWorldOffset` (`self.Cursor`) (`KismetMathLibrary.MakeVector` (`local.MouseX`)) false false)))
      (:`then_1`
        (if (<= (`self.Get Distance` false (`local.MouseY`)) (`self.MaxDistance`))
          (`SceneComponent.K2_AddWorldOffset` (`self.Cursor`) (`KismetMathLibrary.MakeVector` 0.0 (`local.MouseY`)) false false))))
    (elif (> (`self.MaxDistance`) (`KismetMathLibrary.Vector_Distance` (`.Location` (`GameplayStatics.BreakHitResult` _outhit)) (`SceneComponent.K2_GetComponentLocation` (`Actor.RootComponent` (`ActorComponent.GetOwner` (`self.DefaultSceneRoot`))))))
      (`SceneComponent.K2_SetWorldLocation` (`self.Cursor`) (`.Location` (`GameplayStatics.BreakHitResult` _outhit)) false false))))

(fn `UserConstructionScript`)