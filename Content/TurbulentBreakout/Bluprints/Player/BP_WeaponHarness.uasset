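; Player weapon harness that handles picking up, dropping and swapping weapons through Enhanced Input actions.
; Held weapons live in PlayerWeapons and snap-attach to an equipped or holster point, with collision and input toggled on pickup and drop.
; Overlapping a pickup triggers its animation and upgrades the equipped weapon via messages.
; Ammo reaches the HUD after each action and on a looping timer, while another timer prints debug inventory.
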(event `self.ReceiveBeginPlay`
  (`self.EnableInput` (`GameplayStatics.GetPlayerController` 0))
  (`KismetSystemLibrary.K2_SetTimer` null "Ping Ammo Hud" 1.0 true)
  (`KismetSystemLibrary.K2_SetTimer` null "DevOnly" 0.0001 true true))

(event `self.PickupCollider.OnComponentBeginOverlap`
  (params (OverlappedComponent :type "PrimitiveComponent Object Reference") (OtherActor :type "Actor Object Reference") (OtherComp :type "PrimitiveComponent Object Reference") (OtherBodyIndex :type Integer) (bFromSweep :type Boolean) (SweepResult :type "HitResult Structure (by ref)"))
  (if (and (`KismetMathLibrary.ClassIsChildOf` (`GameplayStatics.GetObjectClass` OtherActor) "/Game/TurbulentBreakout/Bluprints/Weapons/WeaponBase/BP_PickupBase.BP_PickupBase_C") (`KismetSystemLibrary.IsValid` (`self.Equiped Weapon`)))
    (`|ExecutionSequence`
      (:`then_0`
        (bind _self_ref (message `/Game/TurbulentBreakout/Bluprints/Interfaces/BPI_Weapon.Get Pickup Self Ref` OtherActor))
        (`/Game/TurbulentBreakout/Bluprints/Weapons/WeaponBase/BP_PickupBase.Pickup Animation` _self_ref))
      (:`then_1`
        (message `/Game/TurbulentBreakout/Bluprints/Interfaces/BPI_Weapon.UpgradeWeapon` OtherActor (`self.Equiped Weapon`))))))

(event `EnhancedInput|/Game/TurbulentBreakout/Bluprints/Input/Actions/IA_ItemSwap`
  (params (ActionValue :type Boolean) (ElapsedSeconds :type "Float (double-precision)") (TriggeredSeconds :type "Float (double-precision)") (InputAction :type "InputAction Object Reference" :default "/Game/TurbulentBreakout/Bluprints/Input/Actions/IA_ItemSwap.IA_ItemSwap"))
  (:`Started`
    (`self.SwapWeapons`)
    (`self.Ping Ammo Hud` :!label _label)))

(event `EnhancedInput|/Game/TurbulentBreakout/Bluprints/Input/Actions/IA_ItemDrop`
  (params (ActionValue :type Boolean) (ElapsedSeconds :type "Float (double-precision)") (TriggeredSeconds :type "Float (double-precision)") (InputAction :type "InputAction Object Reference" :default "/Game/TurbulentBreakout/Bluprints/Input/Actions/IA_ItemDrop.IA_ItemDrop"))
  (:`Started`
    (`self.DropWeapon`)
    (goto _label)))

(event `EnhancedInput|/Game/TurbulentBreakout/Bluprints/Input/Actions/IA_ItemPickup`
  (params (ActionValue :type Boolean) (ElapsedSeconds :type "Float (double-precision)") (TriggeredSeconds :type "Float (double-precision)") (InputAction :type "InputAction Object Reference" :default "/Game/TurbulentBreakout/Bluprints/Input/Actions/IA_ItemPickup.IA_ItemPickup"))
  (:`Started`
    (`self.WeaponPickup`)
    (goto _label)))

(fn `DevOnly`
  (for (_array_element _array_index) (`self.PlayerWeapons`)
    (`KismetSystemLibrary.PrintString` (`KismetSystemLibrary.GetDisplayName` _array_element) true true (struct :`G` 0.66 :`B` 1.0 :`A` 1.0) 0.0)
    (`KismetSystemLibrary.PrintString` (`KismetStringLibrary.Conv_IntToString` _array_index) true true (struct :`R` 0.120794 :`G` 1.0 :`B` 0.213504 :`A` 1.0) 0.0))
  (`KismetSystemLibrary.PrintString` (`KismetSystemLibrary.GetDisplayName` (`self.Equiped Weapon`)) true true (struct :`R` 1.0 :`B` 0.02448 :`A` 1.0) 0.0))

(fn `DropWeapon`
  (if (`KismetSystemLibrary.IsValid` (`self.Equiped Weapon`))
    (for (_array_element _array_index) (`self.PlayerWeapons`)
      (if (== _array_element (`self.Equiped Weapon`))
        (`KismetArrayLibrary.Array_Remove` (`self.PlayerWeapons`) _array_index)
        (break)))
    (`|ExecutionSequence`
      (:`then_0`
        (`SceneComponent.K2_DetachFromComponent` (`Actor.RootComponent` (`self.Equiped Weapon`)) "KeepWorld" "KeepWorld" "KeepWorld" false))
      (:`then_1`
        (`PrimitiveComponent.SetCollisionEnabled` (`/Game/TurbulentBreakout/Bluprints/Weapons/WeaponBase/BP_WeaponBase.Weapon Model` (`self.Equiped Weapon`)) "QueryAndPhysics"))
      (:`then_2`
        (`self.DisableInput` (`self.Equiped Weapon`) (`GameplayStatics.GetPlayerController` 0))
        (set `self.Equiped Weapon` null)))))

(fn `Equip/Unequip`
  (params (Equip :type Boolean) (WeaponRef :type "/Game/TurbulentBreakout/Bluprints/Weapons/WeaponBase/BP_WeaponBase Object Reference"))
  (locals (`Weapon Root` :type "SceneComponent Object Reference"))
  (bind _weaponref (`local.WeaponRef`))
  (if (`KismetSystemLibrary.IsValid` WeaponRef)
    (set `local.Weapon Root` (`Actor.RootComponent` WeaponRef))
    (if Equip
      (`SceneComponent.K2_AttachToComponent` (`local.Weapon Root`) (`self.WeaponEquipedPoint`) "None" "SnapToTarget" "SnapToTarget" "KeepWorld" false)
      (set `/Game/TurbulentBreakout/Bluprints/Weapons/WeaponBase/BP_WeaponBase.Weapon Equipped` true (`local.WeaponRef`))
      (set `self.Equiped Weapon` (`local.WeaponRef`))
      (else
        (`SceneComponent.K2_AttachToComponent` (`local.Weapon Root`) (`self.WeaponHolsterPoint`) "None" "SnapToTarget" "SnapToTarget" "KeepWorld" false)
        (set `/Game/TurbulentBreakout/Bluprints/Weapons/WeaponBase/BP_WeaponBase.Weapon Equipped` false _weaponref)
        (if (== (`self.Equiped Weapon`) _weaponref)
          (set `self.Equiped Weapon` null))))))

(fn `Ping Ammo Hud`
  (if (`KismetSystemLibrary.IsValid` (`self.Equiped Weapon`))
    (message `/Game/TurbulentBreakout/Bluprints/Interfaces/BPI_HUD.Call Update AmmoCounter` (`PlayerController.GetHUD` (`GameplayStatics.GetPlayerController` 0)) (`/Game/TurbulentBreakout/Bluprints/Weapons/WeaponBase/BP_WeaponBase.Weapon Ammo` (`self.Equiped Weapon`)))))

(fn `SwapWeapons`
  (locals (EquipedIndex :type Integer :default -1))
  (bind _output (`|GetArrayItem` (`self.PlayerWeapons`) (`self.MaxIndex`)))
  (bind _output_2 (`|GetArrayItem` (`self.PlayerWeapons`) (- (`local.EquipedIndex`) 1)))
  (for (_array_element _array_index) (`self.PlayerWeapons`)
    (if (`KismetSystemLibrary.IsValid` _array_element)
      (if (== (`self.Equiped Weapon`) _array_element)
        (set `local.EquipedIndex` _array_index)
        (`self.Equip/Unequip` false (`self.Equiped Weapon`))
        (break))))
  (if (and (== (`local.EquipedIndex`) -1) (not (`KismetSystemLibrary.IsValid` (`self.Equiped Weapon`))))
    (for _array_element_2 (`self.PlayerWeapons`)
      (if (`KismetSystemLibrary.IsValid` _array_element_2)
        (`self.Equip/Unequip` true _array_element_2)
        (break)))
    (elif (== (`local.EquipedIndex`) 0)
      (if (`KismetSystemLibrary.IsValid` _output)
        (`self.Equip/Unequip` true _output))
      (elif (`KismetSystemLibrary.IsValid` _output_2)
        (`self.Equip/Unequip` true _output_2)))))

(fn `UserConstructionScript`)

(fn `WeaponPickup`
  (locals (WeaponRef :type "/Game/TurbulentBreakout/Bluprints/Weapons/WeaponBase/BP_WeaponBase Object Reference"))
  (bind _weaponref (`local.WeaponRef`))
  (bind _weaponref_2 (`local.WeaponRef`))
  (bind _weapon_model (`/Game/TurbulentBreakout/Bluprints/Weapons/WeaponBase/BP_WeaponBase.Weapon Model` _weaponref_2))
  (if (< (- (`KismetArrayLibrary.Array_Length` (`self.PlayerWeapons`)) 1) (`self.MaxIndex`))
    (for _array_element (`PrimitiveComponent.GetOverlappingActors` (`self.PickupCollider`) "/Game/TurbulentBreakout/Bluprints/Weapons/WeaponBase/BP_WeaponBase.BP_WeaponBase_C")
      (bind _asbp_weapon_base (cast `/Game/TurbulentBreakout/Bluprints/Weapons/WeaponBase/BP_WeaponBase` _array_element))
      (bind _output_get (set `local.WeaponRef` _asbp_weapon_base))
      (if (`KismetSystemLibrary.IsValid` (`self.Equiped Weapon`))
        (`self.Equip/Unequip` false _output_get)
        (break)
        (else
          (`self.Equip/Unequip` true _output_get)
          (break))))
    (if (`KismetSystemLibrary.IsValid` (`local.WeaponRef`))
      (`KismetArrayLibrary.Array_Add` (`self.PlayerWeapons`) _weaponref_2)
      (if (`KismetSystemLibrary.IsValid` _weapon_model)
        (`PrimitiveComponent.SetCollisionEnabled` _weapon_model "NoCollision")
        (set `/Game/TurbulentBreakout/Bluprints/Weapons/WeaponBase/BP_WeaponBase.Is Player` true _weaponref)
        (`self.EnableInput` _weaponref (`GameplayStatics.GetPlayerController` 0))))))