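; Player character Blueprint for TurbulentBreakout, handling movement, yaw-only look, footsteps and death, with dash, melee and health components.
; Movement input is blocked during a charged dash, and Tick raises spring-arm lag speed while dashing for a tighter follow.
; Holding rotate-camera sends look input to the spring arm instead of controller yaw, then restores its saved rotation on release.
; Debug stat printing and velocity-driven time dilation are present but disconnected.
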(event `EnhancedInput|/Game/TurbulentBreakout/Bluprints/Inputs/Actions/IA_RotateCamera`
  (params (ActionValue :type "Vector2D Structure") (ElapsedSeconds :type "Float (double-precision)") (TriggeredSeconds :type "Float (double-precision)") (InputAction :type "InputAction Object Reference" :default "/Game/TurbulentBreakout/Bluprints/Inputs/Actions/IA_RotateCamera.IA_RotateCamera"))
  (:`Triggered`
    (if (not (`self.Rotating Carmera`))
      (set `self.Rotation` (`SceneComponent.K2_GetComponentRotation` (`self.CameraSprirng`)))
      (set `self.Rotating Carmera` true)))
  (:`Completed`
    (set `self.Rotating Carmera` false)
    (`SceneComponent.K2_SetWorldRotation` (`self.CameraSprirng`) (`self.Rotation`) false false)))

(event `EnhancedInput|/Game/TurbulentBreakout/Bluprints/Inputs/Actions/IA_Look`
  (params (ActionValue :type "Vector2D Structure") (ElapsedSeconds :type "Float (double-precision)") (TriggeredSeconds :type "Float (double-precision)") (InputAction :type "InputAction Object Reference" :default "/Game/TurbulentBreakout/Bluprints/Inputs/Actions/IA_Look.IA_Look"))
  (bind _returnvalue (- (/ ActionValue_X 3.0) (`KismetMathLibrary.Abs` (/ ActionValue_Y 3.0))))
  (:`Triggered`
    (if (`self.Rotating Carmera`)
      (`SceneComponent.K2_AddWorldRotation` (`self.CameraSprirng`) (`KismetMathLibrary.MakeRotator` 0.0 0.0 _returnvalue) false false)
      (else
        (`self.AddControllerYawInput` _returnvalue)))))

(event `self.ReceiveBeginPlay`
  (set `/Game/TurbulentBreakout/Bluprints/Components/CMP_Melee.Attack Range` (`self.Melee Range`) (`self.MeleeComponent`)))

(event `EnhancedInput|/Game/TurbulentBreakout/Bluprints/Inputs/Actions/IA_Movement`
  (params (ActionValue :type "Vector2D Structure") (ElapsedSeconds :type "Float (double-precision)") (TriggeredSeconds :type "Float (double-precision)") (InputAction :type "InputAction Object Reference" :default "/Game/TurbulentBreakout/Bluprints/Inputs/Actions/IA_Movement.IA_Movement"))
  (bind _dashcomponent (`self.DashComponent`))
  (:`Triggered`
    (set `self.Moving?` true)
    (if (not (and (`/Game/TurbulentBreakout/Bluprints/Components/CMP_Dash.Dashing` _dashcomponent) (`/Game/TurbulentBreakout/Bluprints/Components/CMP_Dash.Charged` _dashcomponent)))
      (`self.AddMovementInput` (`self.GetActorRightVector`) ActionValue_X true)
      (`self.AddMovementInput` (`self.GetActorForwardVector`) ActionValue_Y true)
      (`KismetSystemLibrary.Delay` 0.5)
      (if (`self.Moving?`)
        (if (`KismetMathLibrary.RandomBool`)
          (`GameplayStatics.PlaySoundAtLocation` "/Game/TurbulentBreakout/BaseAssets/Sounds/FootStep01.FootStep01" (0.0 0.0 0.0) (struct) 1.0 1.0 0.0 null null null null)
          (else
            (`GameplayStatics.PlaySoundAtLocation` "/Game/TurbulentBreakout/BaseAssets/Sounds/Footstep02.Footstep02" (0.0 0.0 0.0) (struct) 1.0 1.0 0.0 null null null null))))))
  (:`Completed`
    (set `self.Moving?` false)))

(event `/Game/TurbulentBreakout/Bluprints/Interfaces/BPI_Health.Custom DeathEvent`
  (`self.K2_DestroyActor`))

(event `self.ReceiveTick`
  (params (DeltaSeconds :type "Float (single-precision)"))
  (bind _camerasprirng (`self.CameraSprirng`))
  (if (`/Game/TurbulentBreakout/Bluprints/Components/CMP_Dash.Dashing` (`self.DashComponent`))
    (set `SpringArmComponent.CameraLagSpeed` 7.0 _camerasprirng)
    (else
      (set `SpringArmComponent.CameraLagSpeed` 3.0 _camerasprirng))))

(fn `Display Dev Stats`
  (bind (_returnvalue_x _returnvalue_y) (`KismetMathLibrary.BreakVector` (`self.GetVelocity`)))
  (bind _returnvalue_x_2 (`KismetMathLibrary.BreakVector` (`self.GetVelocity`)))
  (`KismetSystemLibrary.PrintString` (`KismetStringLibrary.Conv_DoubleToString` _returnvalue_x_2) true true (struct :`R` 1.0 :`G` 0.864302 :`B` 0.005986 :`A` 1.0) 0.0)
  (`KismetSystemLibrary.PrintString` (`KismetStringLibrary.Conv_DoubleToString` _returnvalue_y) true true (struct :`G` 0.009347 :`B` 1.0 :`A` 1.0) 0.0)
  (`KismetSystemLibrary.PrintString` (`KismetStringLibrary.Conv_DoubleToString` (`/Game/TurbulentBreakout/Bluprints/Components/CMP_Melee.Energy` (`self.MeleeComponent`))) true true (struct :`R` 0.798179 :`G` 0.214249 :`B` 1.0 :`A` 1.0) 0.0)
  (`KismetSystemLibrary.PrintString` (`KismetStringLibrary.Conv_DoubleToString` (`/Game/TurbulentBreakout/Bluprints/Components/CMP_Dash.Energy` (`self.DashComponent`))) true true (struct :`G` 0.66 :`B` 1.0 :`A` 1.0) 0.0)
  (`KismetSystemLibrary.PrintString` (`KismetStringLibrary.Conv_DoubleToString` (`/Game/TurbulentBreakout/Bluprints/Components/CMP_Health.CurrentHealth` (`self.HealthComponment`))) true true (struct :`R` 1.0 :`A` 1.0) 0.0))

(fn `UserConstructionScript`)