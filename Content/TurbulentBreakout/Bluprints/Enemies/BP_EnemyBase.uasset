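; BP_EnemyBase is a base enemy Blueprint that provides shared player-tracking helpers.
; BeginPlay caches the player pawn, its location and the enemy's controller.
; NavigateToPlayer refreshes that location and issues a simple move toward its X/Y, while TraceToPlayer runs a Visibility line trace from the capsule to the cached position.
; AttackPlayer is an empty stub, IsPlayer compares an object to the cached pawn, and nothing here calls these helpers.
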(event `self.ReceiveBeginPlay`
  (bind _returnvalue (`GameplayStatics.GetPlayerPawn` 0))
  (if (`KismetSystemLibrary.IsValid` _returnvalue)
    (bind _output_get (set `self.PlayerRef` _returnvalue))
    (set `self.Player Position` (`self.K2_GetActorLocation` _output_get))
    (set `self.ControllerRef` (`self.GetController` self))))

(fn `AttackPlayer`)

(fn `IsPlayer`
  (params (ObjectRef :type "Object Object Reference"))
  (if (== ObjectRef (`self.PlayerRef`))
    (return)))

(fn `Navigate To Player`
  (bind _playerref (`self.PlayerRef`))
  (if (`KismetSystemLibrary.IsValid` _playerref)
    (bind _output_get (set `self.Player Position` (`self.K2_GetActorLocation` _playerref)))
    (`AIBlueprintHelperLibrary.SimpleMoveToLocation` (`self.ControllerRef`) (`KismetMathLibrary.MakeVector` (.x _output_get) (.y _output_get)))))

(fn `TraceToPlayer`
  (returns (NewParam :type "HitResult Structure"))
  (bind _outhit (`KismetSystemLibrary.LineTraceSingle` (`SceneComponent.K2_GetComponentLocation` (`self.CapsuleComponent`)) (`self.Player Position`) "TraceTypeQuery1"))
  (return _outhit))

(fn `UserConstructionScript`)